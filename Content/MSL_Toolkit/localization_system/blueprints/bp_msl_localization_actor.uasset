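; Localization manager actor that switches text and audio language packs at runtime and serves localized lines, fonts and text-block styling.
; On begin game it builds culture lists from valid archives in the package data table, skipping missing ones.
; Lookups go through nested data tables by archive and line ID, with separate text and audio indices.
; Language changes fire events, collect garbage and notify menu widgets; text changes also set engine culture.
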(event `self.bp_msl_identifier_component.ed_begingame`
  (params (loaded_save_file :type Boolean))
  ;[1 1 1] Localization for changing language packages in runtime,
  ; beginplay is here.
  (`self.init_localization`) ; init all existing localizationg that was found\nin packed content directory,\nshould be called each time localization actor\nreceives beginplay.
)

(event `call_text_changed`
  (params (text_index :type Integer) (culture_id :type String))
  ;[1 1 1] Localization for changing language packages in runtime,
  ; beginplay is here.
  (`self.ed_text_localization_changed` text_index culture_id)
  (`KismetSystemLibrary.CollectGarbage` :!label _label) ; after localization changed,\ngarbage should be removed.
  (bind _foundwidgets (`WidgetBlueprintLibrary.GetAllWidgetsOfClass` "/Game/MSL_Toolkit/menu_system/widgets/base_parent/msl_01_menu_v2.msl_01_menu_v2_C" false))
  (for _array_element _foundwidgets
    (`/Game/MSL_Toolkit/menu_system/widgets/base_parent/msl_01_menu_v2.menu_interact` _array_element "language_changed" "")))

(event `call_audio_changed`
  (params (audio_index :type Integer) (culture_id :type String))
  ;[1 1 1] Localization for changing language packages in runtime,
  ; beginplay is here.
  (`self.ed_audio_localization_changed` audio_index culture_id)
  (goto _label))

(fn `calculate_text_duration`
  (params (text_info :type Text))
  (returns (text_duration :type Integer) (text_length :type Integer))
  (locals (local_text_length :type Integer :default 0) (local_scale :type Integer))
  ;[1 1 1] Calculate text size in case if it is needed,
  ; returns scalar int, from 0 to 7, based on letters count,
  ; can be useful for checking subtitle length, and calculating their duration for reading and etc.
  (set `local.local_text_length` (`KismetStringLibrary.Len` (`KismetTextLibrary.Conv_TextToString` text_info)))
  (`|ExecutionSequence`
    (:`then_0`
      (if (`KismetMathLibrary.InRange_IntInt` (`local.local_text_length`) 0 5)
        (set `local.local_scale` 0)
        (elif (`KismetMathLibrary.InRange_IntInt` (`local.local_text_length`) 5 12)
          (set `local.local_scale` 1)
          (elif (`KismetMathLibrary.InRange_IntInt` (`local.local_text_length`) 5 12)
            (set `local.local_scale` 2)
            (elif (`KismetMathLibrary.InRange_IntInt` (`local.local_text_length`) 12 24)
              (set `local.local_scale` 3)
              (elif (`KismetMathLibrary.InRange_IntInt` (`local.local_text_length`) 24 36)
                (set `local.local_scale` 4)
                (elif (`KismetMathLibrary.InRange_IntInt` (`local.local_text_length`) 36 45)
                  (set `local.local_scale` 5)
                  (elif (`KismetMathLibrary.InRange_IntInt` (`local.local_text_length`) 45 55)
                    (set `local.local_scale` 6)
                    (else
                      (set `local.local_scale` 7))))))))))
    (:`then_1`
      (return (`local.local_scale`) (`local.local_text_length`)))))

(fn `find_localization`
  (params (culture_id :type String) (is_audio :type Boolean) (search_matching :type Boolean))
  (returns (is_valid :type Boolean) (found_id :type String) (found_index :type Integer))
  (locals (local_culture_id :type String) (local_matching_digits :type Integer) (local_culture_chars :type "Array of String") (local_target_chars :type "Array of String") (local_index :type Integer) (local_matching_list :type "Array of Integer") (local_packed_cultures :type "Array of String") (local_found_index :type Integer :default 0))
  (bind _local_culture_chars (`local.local_culture_chars`))
  ;[1 1 1] Find localization by culture ID or find similar in list.
  (set `local.local_culture_id` culture_id)
  (if is_audio
    (set `local.local_packed_cultures` (`self.packaged_cultures_audio`))
    (else
      (set `local.local_packed_cultures` (`self.packaged_cultures_text`))))
  (set `local.local_found_index` (`KismetArrayLibrary.Array_Find` (`local.local_packed_cultures`) (`local.local_culture_id`)))
  (if (>= (`local.local_found_index`) 0)
    (return true (`|GetArrayItem` (`local.local_packed_cultures`) (`local.local_found_index`)) (`local.local_found_index`))
    (else
      (if search_matching
        (set `local.local_target_chars` (`KismetStringLibrary.GetCharacterArrayFromString` (`local.local_culture_id`)))
        (for (_array_element _array_index) (`local.local_packed_cultures`)
          (set `local.local_index` _array_index)
          (set `local.local_culture_chars` (`KismetStringLibrary.GetCharacterArrayFromString` _array_element))
          (for (_array_element_2 _array_index_2) (`local.local_target_chars`) :!label _label
            (if (`KismetArrayLibrary.Array_IsValidIndex` _local_culture_chars _array_index_2)
              (if (`KismetStringLibrary.EqualEqual_StrStr` _array_element_2 (`|GetArrayItem` _local_culture_chars _array_index_2))
                (`/Engine/EditorBlueprintResources/StandardMacros.IncrementInt` (`local.local_matching_digits`)))))
          (`KismetArrayLibrary.Array_Set` (`local.local_matching_list`) (`local.local_index`) (`local.local_matching_digits`) true)
          (set `local.local_matching_digits` 0)
          (goto _label :!via `Break`))
        (set `local.local_found_index` (`KismetMathLibrary.MaxOfIntArray` (`local.local_matching_list`)))
        (if (>= (`local.local_found_index`) 0)
          (return true (`|GetArrayItem` (`local.local_packed_cultures`) (`local.local_found_index`)) (`local.local_found_index`))
          (else
            _)))
      (return false "" 0))))

(fn `get_audio_localization`
  (params (archive_id :type Name) (line_id :type Name))
  (returns (is_valid :type Boolean) (line_audio :type "SoundWave Object Reference") (line_length :type "Float (double-precision)"))
  (locals (local_audio :type "/Game/MSL_Toolkit/localization_system/data/structs/s_loc_info Structure") (local_found :type Boolean))
  (bind (_line_text _line_sound _line_length) (break `/Game/MSL_Toolkit/localization_system/data/structs/s_loc_info` (`local.local_audio`)))
  ;[1 1 1] get any audio localization from archive and line ID, and also does check if localization does exist.
  (`|ExecutionSequence`
    (:`then_0`
      (if (>= (`self.audio_index`) 0)
        (if (`KismetArrayLibrary.Array_IsValidIndex` (`self.packaged_localizations_audio`) (`self.audio_index`))
          (bind _returnvalue (`|GetDataTableRow` (`|GetArrayItem` (`self.packaged_localizations_audio`) (`self.audio_index`)) archive_id)
            (:`then`
              (bind _localization_data (break `/Game/MSL_Toolkit/localization_system/data/structs/s_loc_archive` _returnvalue))
              (if (`KismetSystemLibrary.IsValid` _localization_data)
                (bind _returnvalue_2 (`|GetDataTableRow` _localization_data line_id)
                  (:`then`
                    (set `local.local_audio` _returnvalue_2)
                    (set `local.local_found` true)))))))))
    (:`then_1`
      (return (and (`local.local_found`) (`KismetSystemLibrary.IsValid` _line_sound)) _line_sound _line_length) ; return audio file and\ninfo about validness.
    )))

(fn `get_font`
  (params (font_family :type Name) (font_typeface :type Name) (font_size :type Integer :default 0))
  (returns (SlateFontInfo :type "SlateFontInfo Structure"))
  (bind _returnvalue (`KismetMathLibrary.SelectInt` font_size 24 (>= font_size 1)))
  ;[1 1 1] Get specific font from data, with custom or default size,
  ; if font is not found, return default font with custom size or default size.
  (bind _returnvalue_2 (`|GetDataTableRow` "/Game/MSL_Toolkit/localization_system/common/msl_loc_fonts_data.msl_loc_fonts_data" font_family) ; check if font family is found inside datatable.
    (:`then`
      (return (make `SlateFontInfo` (`.font_family_2_B9C339F242B40B0A3BD403B64AE6435A` (break `/Game/MSL_Toolkit/localization_system/data/structs/s_loc_font` _returnvalue_2)) null (struct :`OutlineColor` (struct :`A` 1.0)) font_typeface _returnvalue)) ; if so return valid font data.
    )
    (:`RowNotFound`
      (return (make `SlateFontInfo` "/Game/MSL_Toolkit/localization_system/data/fonts/roboto/Roboto.Roboto" null (struct :`OutlineColor` (struct :`A` 1.0)) font_typeface _returnvalue)) ; if no valid data,\nreturn default font.
    )))

(fn `get_line_data`
  (params (archive_id :type Name) (line_id :type Name))
  (returns (is_found_text :type Boolean) (is_found_audio :type Boolean) (text_data :type "/Game/MSL_Toolkit/localization_system/data/structs/s_loc_info Structure") (audio_data :type "/Game/MSL_Toolkit/localization_system/data/structs/s_loc_info Structure"))
  (locals (local_archive_id :type Name) (local_line_id :type Name) (local_text_data :type "/Game/MSL_Toolkit/localization_system/data/structs/s_loc_info Structure") (local_text_found :type Boolean) (local_audio_data :type "/Game/MSL_Toolkit/localization_system/data/structs/s_loc_info Structure") (local_audio_found :type Boolean))
  ;[1 1 1] get default line data, both audio and text if found,
  ; returns data instead of text/audio and etc.
  (set `local.local_archive_id` archive_id)
  (set `local.local_line_id` line_id)
  (`|ExecutionSequence`
    (:`then_0`
      (if (>= (`self.text_index`) 0)
        (if (`KismetArrayLibrary.Array_IsValidIndex` (`self.packaged_localizations_text`) (`self.text_index`))
          (bind _returnvalue (`|GetDataTableRow` (`|GetArrayItem` (`self.packaged_localizations_text`) (`self.text_index`)) (`local.local_archive_id`))
            (:`then`
              (bind _localization_data (break `/Game/MSL_Toolkit/localization_system/data/structs/s_loc_archive` _returnvalue))
              (if (`KismetSystemLibrary.IsValid` _localization_data)
                (bind _returnvalue_2 (`|GetDataTableRow` _localization_data (`local.local_line_id`))
                  (:`then`
                    (set `local.local_text_data` _returnvalue_2)
                    (set `local.local_text_found` true)))))))))
    (:`then_1`
      (if (>= (`self.audio_index`) 0)
        (if (`KismetArrayLibrary.Array_IsValidIndex` (`self.packaged_localizations_audio`) (`self.audio_index`))
          (bind _returnvalue_3 (`|GetDataTableRow` (`|GetArrayItem` (`self.packaged_localizations_audio`) (`self.audio_index`)) (`local.local_archive_id`))
            (:`then`
              (bind _localization_data_2 (break `/Game/MSL_Toolkit/localization_system/data/structs/s_loc_archive` _returnvalue_3))
              (if (`KismetSystemLibrary.IsValid` _localization_data_2)
                (bind _returnvalue_4 (`|GetDataTableRow` _localization_data_2 (`local.local_line_id`))
                  (:`then`
                    (set `local.local_audio_data` _returnvalue_4)
                    (set `local.local_audio_found` true)))))))))
    (:`then_2`
      (return false false (`local.local_text_data`) (`local.local_audio_data`)))))

(fn `get_line_localization`
  (params (archive_id :type Name) (line_id :type Name))
  (returns (is_valid_text :type Boolean) (is_valid_audio :type Boolean) (line_from_data :type Boolean) (line_text :type Text) (line_file :type "SoundWave Object Reference") (line_length :type "Float (double-precision)") (line_scale :type Integer))
  (locals (local_archive_id :type Name) (local_line_id :type Name) (local_text_data :type "/Game/MSL_Toolkit/localization_system/data/structs/s_loc_info Structure") (local_text_found :type Boolean) (local_audio_data :type "/Game/MSL_Toolkit/localization_system/data/structs/s_loc_info Structure") (local_audio_found :type Boolean))
  (bind (_line_text _line_sound _line_length) (break `/Game/MSL_Toolkit/localization_system/data/structs/s_loc_info` (`local.local_audio_data`)))
  (bind (_line_text_2 _line_sound_2 _line_length_2 _line_scale) (break `/Game/MSL_Toolkit/localization_system/data/structs/s_loc_info` (`local.local_text_data`)))
  (bind (_line_text_3 _line_sound_3 _line_length_3 _line_scale_2) (break `/Game/MSL_Toolkit/localization_system/data/structs/s_loc_info` (`local.local_audio_data`)))
  (bind _returnvalue (`KismetTextLibrary.Conv_NameToText` (`local.local_line_id`)))
  ;[1 1 1] Get more versatile localization with both text and audio,
  ; reads separate channels of current audio and current text,
  ; and returns both.
  (set `local.local_archive_id` archive_id)
  (set `local.local_line_id` line_id)
  (`|ExecutionSequence`
    (:`then_0`
      (if (>= (`self.text_index`) 0)
        (if (`KismetArrayLibrary.Array_IsValidIndex` (`self.packaged_localizations_text`) (`self.text_index`))
          (bind _returnvalue_2 (`|GetDataTableRow` (`|GetArrayItem` (`self.packaged_localizations_text`) (`self.text_index`)) (`local.local_archive_id`))
            (:`then`
              (bind _localization_data (break `/Game/MSL_Toolkit/localization_system/data/structs/s_loc_archive` _returnvalue_2))
              (if (`KismetSystemLibrary.IsValid` _localization_data)
                (bind _returnvalue_3 (`|GetDataTableRow` _localization_data (`local.local_line_id`))
                  (:`then`
                    (set `local.local_text_data` _returnvalue_3)
                    (set `local.local_text_found` true)))))))))
    (:`then_1`
      (if (>= (`self.audio_index`) 0)
        (if (`KismetArrayLibrary.Array_IsValidIndex` (`self.packaged_localizations_audio`) (`self.audio_index`))
          (bind _returnvalue_4 (`|GetDataTableRow` (`|GetArrayItem` (`self.packaged_localizations_audio`) (`self.audio_index`)) (`local.local_archive_id`))
            (:`then`
              (bind _localization_data_2 (break `/Game/MSL_Toolkit/localization_system/data/structs/s_loc_archive` _returnvalue_4))
              (if (`KismetSystemLibrary.IsValid` _localization_data_2)
                (bind _returnvalue_5 (`|GetDataTableRow` _localization_data_2 (`local.local_line_id`))
                  (:`then`
                    (set `local.local_audio_data` _returnvalue_5)
                    (set `local.local_audio_found` true)))))))))
    (:`then_2`
      (if (`local.local_text_found`)
        (return (not (`KismetTextLibrary.TextIsEmpty` _line_text_2)) (and (`local.local_audio_found`) (`KismetSystemLibrary.IsValid` _line_sound)) (`local.local_text_found`) _line_text_2 _line_sound _line_length _line_scale)
        (else
          (return (not (`KismetTextLibrary.TextIsEmpty` _returnvalue)) (and (`local.local_audio_found`) (`KismetSystemLibrary.IsValid` _line_sound_3)) (`local.local_text_found`) _returnvalue _line_sound_3 _line_length_3 _line_scale_2))))))

(fn `get_text_localization`
  (params (archive_id :type Name) (line_id :type Name))
  (returns (is_valid :type Boolean) (from_data :type Boolean) (line_text :type Text) (line_scale :type Integer))
  ;[1 1 1] get the localized text from archive and line, and check if the localization and the text itself exist.
  ; we also do check if text is numeric is so we will return the valid text.
  (if (>= (`self.text_index`) 0)
    (if (`KismetArrayLibrary.Array_IsValidIndex` (`self.packaged_localizations_text`) (`self.text_index`))
      (bind _returnvalue (`|GetDataTableRow` (`|GetArrayItem` (`self.packaged_localizations_text`) (`self.text_index`)) archive_id)
        (:`then`
          (bind _localization_data (break `/Game/MSL_Toolkit/localization_system/data/structs/s_loc_archive` _returnvalue))
          (if (`KismetSystemLibrary.IsValid` _localization_data)
            (bind _returnvalue_2 (`|GetDataTableRow` _localization_data line_id)
              (:`then`
                (bind (_line_text _line_sound _line_length _line_scale) (break `/Game/MSL_Toolkit/localization_system/data/structs/s_loc_info` _returnvalue_2))
                (return (not (`KismetTextLibrary.TextIsEmpty` _line_text)) true _line_text _line_scale) ; return that text is not valid\nif its empty.
              )
              (:`RowNotFound`
                (return true false (`KismetTextLibrary.Conv_NameToText` line_id) 0) ; if row not found,\nreturn the ID as text.
              ))
            (else
              (return false false "#DATA NOT FOUND#" 0) ; if data not found,\nreturn info about that.
            )))
        (:`RowNotFound`
          (return false false "#ARCHIVE NOT FOUND#" 0) ; if archive not found,\nreturn info about that.
        ))
      (else
        _)))
  (return false false "#LANGUAGE NOT FOUND#" 0) ; if language is not found,\nreturn info about that.
)

(fn `init_localization`
  ;[1 1 1] Initiate the localization data and fill the existing data from files.
  ; We are loading only existing localization tables from content folder by validation check,
  ; So if some of the languages are gets deleted it will not cause any issues, just that localization will be ignored.
  (`|ExecutionSequence`
    (:`then_0`
      (`KismetArrayLibrary.Array_Clear` (`self.packaged_cultures_text`))
      (`KismetArrayLibrary.Array_Clear` (`self.packaged_cultures_audio`))
      (`KismetArrayLibrary.Array_Clear` (`self.packaged_localizations_text`))
      (`KismetArrayLibrary.Array_Clear` (`self.packaged_localizations_audio`)))
    (:`then_1`
      (bind _outrownames (`DataTableFunctionLibrary.GetDataTableRowNames` "/Game/MSL_Toolkit/localization_system/common/msl_loc_package_data.msl_loc_package_data")) ; get data about packaged localizations.
      (for _array_element _outrownames
        (bind _returnvalue (`|GetDataTableRow` "/Game/MSL_Toolkit/localization_system/common/msl_loc_package_data.msl_loc_package_data" _array_element) ; get all its rows and add as language datas.
          (:`then`
            (bind (_culture_id _loc_archive_text _loc_archive_audio) (break `/Game/MSL_Toolkit/localization_system/data/structs/s_loc_package` _returnvalue))
            (if (`KismetSystemLibrary.IsValid` _loc_archive_text)
              (`KismetArrayLibrary.Array_Add` (`self.packaged_cultures_text`) _culture_id)
              (`KismetArrayLibrary.Array_Add` (`self.packaged_localizations_text`) _loc_archive_text))
            (if (`KismetSystemLibrary.IsValid` _loc_archive_audio)
              (`KismetArrayLibrary.Array_Add` (`self.packaged_cultures_audio`) _culture_id)
              (`KismetArrayLibrary.Array_Add` (`self.packaged_localizations_audio`) _loc_archive_audio))))))))

(fn `set_audio_localization`
  (params (culture_index :type Integer))
  (bind _packaged_cultures_audio (`self.packaged_cultures_audio`))
  ;[1 1 1] set the audio localization if the culture does not exist set the first index of audio culture that does exist.
  (if (`KismetArrayLibrary.Array_IsValidIndex` _packaged_cultures_audio culture_index)
    (set `self.audio_culture` (`|GetArrayItem` _packaged_cultures_audio culture_index))
    (set `self.audio_index` culture_index)
    (`self.call_audio_changed` (`self.audio_index`) (`self.audio_culture`) :!label _label)
    (elif (`KismetArrayLibrary.Array_IsValidIndex` _packaged_cultures_audio)
      (set `self.audio_culture` (`|GetArrayItem` _packaged_cultures_audio))
      (set `self.audio_index` 0)
      (goto _label))))

(fn `set_text_localization`
  (params (culture_index :type Integer))
  (bind _packaged_cultures_text (`self.packaged_cultures_text`))
  ;[1 1 1] Set text localization by culture index, if there is no such valid index we will load the first index if it exist.
  ; Also after loading the culture we notificate all the UI and Menus about that, so they can update.
  (if (`KismetArrayLibrary.Array_IsValidIndex` _packaged_cultures_text culture_index)
    (bind _output_get (set `self.text_culture` (`|GetArrayItem` _packaged_cultures_text culture_index)))
    (`KismetInternationalizationLibrary.SetCurrentCulture` _output_get true) ; set engine culture and save to config.
    (set `self.text_index` culture_index)
    (`self.call_text_changed` (`self.text_index`) (`self.text_culture`) :!label _label)
    (elif (`KismetArrayLibrary.Array_IsValidIndex` _packaged_cultures_text)
      (bind _output_get_2 (set `self.text_culture` (`|GetArrayItem` _packaged_cultures_text)))
      (`KismetInternationalizationLibrary.SetCurrentCulture` _output_get_2 true) ; set engine culture and save to config.
      (set `self.text_index` 0)
      (goto _label))))

(fn `set_textblock`
  (params (text_reference :type "Object Object Reference") (text_info :type Text) (font_info :type "SlateFontInfo Structure"))
  (locals (local_empty_font :type "Array of SlateFontInfo Structure") (local_text :type Text) (local_font :type "SlateFontInfo Structure"))
  (bind (_fontobject _fontmaterial _outlinesettings _typefacefontname _size) (break `SlateFontInfo` (`local.local_font`)))
  ;[1 1 1] Just an easy function to localize text block with reference text and font info,
  ; If font info is empty font will be not changed.
  (set `local.local_text` text_info)
  (set `local.local_font` font_info)
  (bind _astext (cast `TextBlock` text_reference)) ; find text block reference.
  (`TextBlock.SetText` _astext (`local.local_text`)) ; set its text.
  (if (not (`KismetArrayLibrary.Array_Contains` (`local.local_empty_font`) (`local.local_font`)))
    (bind _structout (setmembers `SlateFontInfo` :`StructRef` (`TextBlock.Font` _astext) :`FontObject` _fontobject :`TypefaceFontName` _typefacefontname :`Size` _size))
    (`TextBlock.SetFont` _astext _structout)))

(fn `UserConstructionScript`)