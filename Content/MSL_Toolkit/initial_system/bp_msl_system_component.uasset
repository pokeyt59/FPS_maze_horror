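; Player controller component that bootstraps the MSL Toolkit system on BeginPlay, intended as a separate client-side copy per player.
; InitSpawn spawns localization, settings, menu and savegame actors where none exist, storing references only to those it spawns, then flags the system loaded.
; It then binds to the menu and settings actors, re-broadcasting device-changed and settings-updated events through its own dispatchers.
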(event `self.ReceiveBeginPlay`
  ;[1 1 1] This component should spawn all important actors with game start,
  ; should be added to player controller only.
  ; beginplay is here.
  (`self.init_system`) ; this is only client sided call,\nbecause each client should have its own copy of system.
)

(event `init_system`
  ;[1 1 1] This component should spawn all important actors with game start,
  ; should be added to player controller only.
  ; beginplay is here.
  (`|ExecutionSequence`
    (:`then_0`
      (`self.init_spawn`))
    (:`then_1`
      (`/Engine/EditorBlueprintResources/StandardMacros.IsValid` (`self.menu_actor`)
        (:`Is Valid`
          (add `/Game/MSL_Toolkit/menu_system/blueprints/bp_msl_menu_actor.ed_device_changed` (`self.menu_actor`) (delegate `call_device_changed`)))))
    (:`then_2`
      (`/Engine/EditorBlueprintResources/StandardMacros.IsValid` (`self.settings_actor`)
        (:`Is Valid`
          (add `/Game/MSL_Toolkit/settings_system/blueprints/bp_msl_settings_actor.ed_settings_updated` (`self.settings_actor`) (delegate `call_settings_updated`)))))))

(event `call_device_changed`
  (params (gamepad :type Boolean))
  ;[1 1 1] This component should spawn all important actors with game start,
  ; should be added to player controller only.
  ; beginplay is here.
  (`self.ed_device_changed` gamepad))

(event `call_settings_updated`
  (params (settings_name :type Name) (settings_value :type Integer) (slider_value :type "Float (double-precision)") (is_slider :type Boolean) (is_apply :type Boolean))
  ;[1 1 1] This component should spawn all important actors with game start,
  ; should be added to player controller only.
  ; beginplay is here.
  (`self.ed_settings_updated` settings_name settings_value slider_value is_slider is_apply))

(fn `init_spawn`
  (locals (local_transform :type "Transform Structure"))
  ;[1 1 1] This actor should init system and load all actors.
  (`|ExecutionSequence`
    (:`then_0`
      (`|ExecutionSequence`
        (:`then_0`
          (bind _outactors (`GameplayStatics.GetAllActorsOfClass` "/Game/MSL_Toolkit/localization_system/blueprints/bp_msl_localization_actor.bp_msl_localization_actor_C"))
          (if (not (`KismetArrayLibrary.Array_IsValidIndex` _outactors))
            (bind _returnvalue (`|SpawnActorFromClass` "/Game/MSL_Toolkit/localization_system/blueprints/bp_msl_localization_actor.bp_msl_localization_actor_C" (`local.local_transform`) "AlwaysSpawn" "OverrideRootScale" null null))
            (set `self.localization_actor` _returnvalue)))
        (:`then_1`
          (bind _outactors_2 (`GameplayStatics.GetAllActorsOfClass` "/Game/MSL_Toolkit/settings_system/blueprints/bp_msl_settings_actor.bp_msl_settings_actor_C"))
          (if (not (`KismetArrayLibrary.Array_IsValidIndex` _outactors_2))
            (bind _returnvalue_2 (`|SpawnActorFromClass` "/Game/MSL_Toolkit/settings_system/blueprints/bp_msl_settings_actor.bp_msl_settings_actor_C" (`local.local_transform`) "AlwaysSpawn" "OverrideRootScale" null null))
            (set `self.settings_actor` _returnvalue_2)))
        (:`then_2`
          (bind _outactors_3 (`GameplayStatics.GetAllActorsOfClass` "/Game/MSL_Toolkit/menu_system/blueprints/bp_msl_menu_actor.bp_msl_menu_actor_C"))
          (if (not (`KismetArrayLibrary.Array_IsValidIndex` _outactors_3))
            (bind _returnvalue_3 (`|SpawnActorFromClass` "/Game/MSL_Toolkit/menu_system/blueprints/bp_msl_menu_actor.bp_msl_menu_actor_C" (`local.local_transform`) "AlwaysSpawn" "OverrideRootScale" null null))
            (set `self.menu_actor` _returnvalue_3)))
        (:`then_3`
          (bind _outactors_4 (`GameplayStatics.GetAllActorsOfClass` "/Game/MSL_Toolkit/savegame_system/blueprints/bp_msl_savegame_actor.bp_msl_savegame_actor_C"))
          (if (not (`KismetArrayLibrary.Array_IsValidIndex` _outactors_4))
            (bind _returnvalue_4 (`|SpawnActorFromClass` "/Game/MSL_Toolkit/savegame_system/blueprints/bp_msl_savegame_actor.bp_msl_savegame_actor_C" (`local.local_transform`) "AlwaysSpawn" "OverrideRootScale" null null))
            (set `self.savegame_actor` _returnvalue_4)))))
    (:`then_1`
      (set `self.is_system_loaded` true) ; after all necessary actors are spawned,\nand all objects is loaded from save file and etc,\nwe should mark the system as loaded.
    )))