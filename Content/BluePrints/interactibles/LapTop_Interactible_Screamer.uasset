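; Laptop interactible that acts as an audio scare, playing a screaming sound when its trigger box is overlapped.
; Box overlap plays Insane_Screaming at the Model component's location, with no actor filter or one-shot guard.
; The construction script primes that cue, two other cues and two empty slots, re-running the parent construction script after each.
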(event `self.Box.OnComponentHit`
  (params (HitComponent :type "PrimitiveComponent Object Reference") (OtherActor :type "Actor Object Reference") (OtherComp :type "PrimitiveComponent Object Reference") (NormalImpulse :type "Vector Structure") (Hit :type "HitResult Structure (by ref)")))

(event `self.Box.OnComponentBeginOverlap`
  (params (OverlappedComponent :type "PrimitiveComponent Object Reference") (OtherActor :type "Actor Object Reference") (OtherComp :type "PrimitiveComponent Object Reference") (OtherBodyIndex :type Integer) (bFromSweep :type Boolean) (SweepResult :type "HitResult Structure (by ref)"))
  (`GameplayStatics.PlaySoundAtLocation` "/Game/sound_design/Insane_Screaming.Insane_Screaming" (`SceneComponent.K2_GetComponentLocation` (`self.model`)) (struct) 1.0 1.0 0.0 null null null))

(fn `UserConstructionScript`
  (`|ExecutionSequence`
    (:`then_0`
      (`AudioMixerBlueprintLibrary.PrimeSoundCueForPlayback` "/Game/sound_design/Insane_Screaming.Insane_Screaming"))
    (:`then_1`
      (`AudioMixerBlueprintLibrary.PrimeSoundCueForPlayback` "/Game/sound_design/KYS_Sound_TEST.KYS_Sound_TEST"))
    (:`then_2`
      (`AudioMixerBlueprintLibrary.PrimeSoundCueForPlayback` "/Game/StarterContent/Audio/Smoke01_Cue.Smoke01_Cue"))
    (:`then_3`
      (`AudioMixerBlueprintLibrary.PrimeSoundCueForPlayback` null))
    (:`then_4`
      (`AudioMixerBlueprintLibrary.PrimeSoundCueForPlayback` null)))
  (`parent.UserConstructionScript`))