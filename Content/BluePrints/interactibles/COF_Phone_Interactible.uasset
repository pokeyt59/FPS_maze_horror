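; COF_Phone_Interactible is an interactable phone actor that hurts the player when used.
; Its construction script primes a test sound cue, which Interact then plays loudly, attached to the Cof component.
; Interact then casts the first player character to Player_v4, subtracts a fixed amount of Health clamped between zero and MaxHealth, and destroys the actor.
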(event `self.ReceiveBeginPlay`)

(fn `interact`
  (returns (`Did Interact?` :type Boolean))
  (`GameplayStatics.SpawnSoundAttached` "/Game/sound_design/KYS_Sound_TEST.KYS_Sound_TEST" (`self.cof`) "None" (0.0 0.0 0.0) (struct) "KeepRelativeOffset" false 4.0 1.0 0.0 null null)
  ;[1 1 1] damage player then disapear
  (bind _asplayer_v_4 (cast `/Game/Player/BluePrint/Player_v4` (`GameplayStatics.GetPlayerCharacter` 0)))
  (set `/Game/Player/BluePrint/Player_v4.Health` (`KismetMathLibrary.Clamp` (- (`/Game/Player/BluePrint/Player_v4.Health` _asplayer_v_4) 20) 0 (`/Game/Player/BluePrint/Player_v4.MaxHealth` _asplayer_v_4)) _asplayer_v_4)
  (`self.K2_DestroyActor`)
  (return true))

(fn `UserConstructionScript`
  (`AudioMixerBlueprintLibrary.PrimeSoundCueForPlayback` "/Game/sound_design/KYS_Sound_TEST.KYS_Sound_TEST"))