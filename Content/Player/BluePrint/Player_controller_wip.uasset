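; Work-in-progress player Blueprint that handles first-person input and survival stats, acting on the character through PlayerRef.
; Input events drive movement, look, jump, sprint, flashlight and a test animation, while crouch halves walk speed and lerps capsule height on a Timeline.
; Stamina drain, stamina regen and health regen are self-recalling Delay loops, with a heartbeat sound at low health.
; Interact line-traces from the camera and messages actors implementing Interaction_Interface.
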(event `Drain Stamina`
  (bind _player_ref (`self.player_ref`))
  (bind _player_ref_2 (`self.player_ref`))
  ;[1 0.2542 0] Stamina system
  ;;[1 0.2542 0] Stamina Drain
  (bind _output_get (set `/Game/Player/BluePrint/Player_v4.Stamina` (`KismetMathLibrary.Clamp` (- (`/Game/Player/BluePrint/Player_v4.Stamina` _player_ref_2) 1) 0 (`/Game/Player/BluePrint/Player_v4.MaxStamina` _player_ref_2)) _player_ref))
  (if (== _output_get 0)
    (`/Game/Player/BluePrint/Player_v4.StopSprinting` _player_ref)
    (elif (`/Game/Player/BluePrint/Player_v4.IsSprinting?` _player_ref_2)
      (`KismetSystemLibrary.Delay` 0.3)
      (`/Game/Player/BluePrint/Player_v4.Drain Stamina` _player_ref_2))))

(event `InputAxis|LookUp/LookDown`
  (params (AxisValue :type "Float (single-precision)"))
  ;[1 1 1] Camera Rotation
  (`Pawn.AddControllerPitchInput` (`self.player_ref`) (`KismetMathLibrary.FClamp` AxisValue -1000.0)))

(event `InputAction|jump`
  (params (Key :type "Key Structure"))
  (bind _player_ref (`self.player_ref`))
  ;[1 1 1] Special actions
  ;;[1 1 1] jumping
  (:`Pressed`
    (if (`NavMovementComponent.IsMovingOnGround` (`Character.CharacterMovement` _player_ref))
      (`Character.Jump` _player_ref))))

(event `InputAxis|LookRight/LookLeft`
  (params (AxisValue :type "Float (single-precision)"))
  ;[1 1 1] Camera Rotation
  (`Pawn.AddControllerYawInput` (`self.player_ref`) (`KismetMathLibrary.FClamp` AxisValue -100.0 100.0)))

(event `InputAction|Crouch`
  (params (Key :type "Key Structure"))
  (bind _player_ref (`self.player_ref`))
  (bind _charactermovement (`Character.CharacterMovement` _player_ref))
  (bind _walkspeed (`/Game/Player/BluePrint/Player_v4.WalkSpeed` _player_ref))
  ;[1 1 1] Special actions
  ;;[1 1 1] Crouch
  (:`Pressed`
    (set `CharacterMovementComponent.MaxWalkSpeed` (/ _walkspeed 2.0) _charactermovement) ; slows down speed for crouching
    (bind (_direction _crouch) (`Timeline|Timeline_1` :!label _label)
      (:`Update`
        (`CapsuleComponent.SetCapsuleHalfHeight` (`Character.CapsuleComponent` _player_ref) (`KismetMathLibrary.Lerp` 91.0 45.5 _crouch) true))))
  (:`Released`
    (set `CharacterMovementComponent.MaxWalkSpeed` _walkspeed _charactermovement)
    (goto _label :!via `Reverse`)))

(event `RegenStamina`
  (bind _player_ref (`self.player_ref`))
  (bind _maxstamina (`/Game/Player/BluePrint/Player_v4.MaxStamina` _player_ref))
  ;[1 0.2542 0] Stamina system
  ;;[1 0.2542 0] Stamina Regen
  (bind _output_get (set `/Game/Player/BluePrint/Player_v4.Stamina` (`KismetMathLibrary.Clamp` (+ (`/Game/Player/BluePrint/Player_v4.Stamina` _player_ref) (`/Game/Player/BluePrint/Player_v4.StaminaRegenRate` _player_ref)) 0 _maxstamina) _player_ref))
  (if (== _output_get _maxstamina)
    _
    (elif (not (`/Game/Player/BluePrint/Player_v4.IsSprinting?` _player_ref))
      (`KismetSystemLibrary.Delay` 0.4)
      (`/Game/Player/BluePrint/Player_v4.RegenStamina` _player_ref))))

(event `InputAxis|MoveLeft/Right`
  (params (AxisValue :type "Float (single-precision)"))
  ;[1 1 1] movement
  (`Pawn.AddMovementInput` (`self.player_ref`) (`self.GetActorRightVector`) AxisValue false))

(event `InputAxis|MoveFoward/Back`
  (params (AxisValue :type "Float (single-precision)"))
  ;[1 1 1] movement
  (`Pawn.AddMovementInput` (`self.player_ref`) (`self.GetActorForwardVector`) AxisValue false))

(event `InputAction|Flashlight On/Off`
  (params (Key :type "Key Structure"))
  (bind _player_ref (`self.player_ref`))
  ;[1 0.9398 0.3352] Flashlight toggle
  (:`Pressed`
    (`SceneComponent.SetVisibility` (`/Game/Player/BluePrint/Player_v4.SpotLight1` _player_ref) (not (`SceneComponent.IsVisible` (`/Game/Player/BluePrint/Player_v4.SpotLight` _player_ref))) false)
    (`SceneComponent.SetVisibility` (`/Game/Player/BluePrint/Player_v4.SpotLight` _player_ref) (not (`SceneComponent.IsVisible` (`/Game/Player/BluePrint/Player_v4.SpotLight` _player_ref))) false)
    (`GameplayStatics.PlaySound2D` "/Game/Movies/Audio/flashlight-on.flashlight-on" 4.0 1.0 0.0 null null)))

(event `InputAction|jump`
  (params (Key :type "Key Structure"))
  (bind _player_ref (`self.player_ref`))
  ;[1 1 1] jumping
  (:`Pressed`
    (if (`NavMovementComponent.IsMovingOnGround` (`Character.CharacterMovement` _player_ref))
      (`Character.Jump` _player_ref))))

(event `InputAction|sprint`
  (params (Key :type "Key Structure"))
  (bind _player_ref (`self.player_ref`))
  ;[1 1 1] movement
  ;;[1 1 1] Special movement
  (:`Pressed`
    (`/Game/Player/BluePrint/Player_v4.StartSprinting` _player_ref))
  (:`Released`
    (`/Game/Player/BluePrint/Player_v4.StopSprinting` _player_ref)))

(event `InputAction|interact`
  (params (Key :type "Key Structure"))
  (bind _camera (`/Game/Player/BluePrint/Player_v4.Camera` (`self.player_ref`)))
  (bind _returnvalue (`SceneComponent.K2_GetComponentLocation` _camera))
  ;[1 1 1] interaction system
  (:`Pressed`
    (bind (_outhit _returnvalue_2) (`KismetSystemLibrary.LineTraceSingle` :`Start` _returnvalue :`End` (+ _returnvalue (* (`SceneComponent.GetForwardVector` _camera) 250.0)) :`TraceChannel` "TraceTypeQuery1" :`DrawDebugType` "ForDuration"))
    (if _returnvalue_2
      (bind (_bblockinghit _binitialoverlap _time _distance _location _impactpoint _normal _impactnormal _physmat _hitactor) (`GameplayStatics.BreakHitResult` _outhit))
      (if (`KismetSystemLibrary.DoesImplementInterface` _hitactor "/Game/BluePrints/Interface/Interaction_Interface.Interaction_Interface_C")
        (message `/Game/BluePrints/Interface/Interaction_Interface.interact` _hitactor)))))

(event `RegenHealth`
  (bind _player_ref (`self.player_ref`))
  ;[1 0 0.02416] Health regen
  (set `/Game/Player/BluePrint/Player_v4.Is Healing?` true _player_ref)
  (bind _output_get (set `/Game/Player/BluePrint/Player_v4.Health` (`KismetMathLibrary.Clamp` (+ (`/Game/Player/BluePrint/Player_v4.Health` _player_ref) (`/Game/Player/BluePrint/Player_v4.HealthRegenRate` _player_ref)) 0 (`/Game/Player/BluePrint/Player_v4.MaxHealth` _player_ref)) _player_ref))
  (if (not (== _output_get 0))
    (set `/Game/Player/BluePrint/Player_v4.Is Healing?` false _player_ref)
    (`|ExecutionSequence`
      (:`then_0`
        (`KismetSystemLibrary.Delay` 0.5)
        (`/Game/Player/BluePrint/Player_v4.RegenHealth` _player_ref))
      (:`then_1`
        ;[1 1 1] your dieing peater
        (`KismetSystemLibrary.Delay` 1.0)
        (if (<= (`/Game/Player/BluePrint/Player_v4.Health` _player_ref) 20)
          (set `/Game/Player/BluePrint/Player_v4.Is Critical condition?` true _player_ref)
          (`GameplayStatics.PlaySound2D` "/Game/Movies/Audio/COF_SOUNDS/heartbeat_Critical_Health.heartbeat_Critical_Health" 1.0 1.0 0.0 null null)
          (else
            (set `/Game/Player/BluePrint/Player_v4.Is Critical condition?` true _player_ref)))))))

(event `InputAction|player animation test 1`
  (params (Key :type "Key Structure"))
  (bind _rp_eric_rigged_001_ue4 (`/Game/Player/BluePrint/Player_v4.rp_eric_rigged_001_ue4` (`self.player_ref`)))
  ;[1 1 1] basic animation controll
  (:`Pressed`
    (`KismetSystemLibrary.PrintString` "is animating")
    (`SkeletalMeshComponent.PlayAnimation` _rp_eric_rigged_001_ue4 "/Game/Player/animations/Holding_Idle_mirror_mixamo_com.Holding_Idle_mirror_mixamo_com" true))
  (:`Released`
    (`KismetSystemLibrary.PrintString` "is't animating")
    (`SkeletalMeshComponent.Stop` _rp_eric_rigged_001_ue4)))

(fn `UserConstructionScript`)