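; Flashlight actor Blueprint with two spot lights and a point light, switched through an Interact function.
; Interact uses a FlipFlop to hide and unhide the actor that owns the lights on alternate calls, then returns true.
; It sets visibility on each light's owner rather than on the light components, and the event graph runs no logic.
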(fn `interact`
  (returns (`Did Interact?` :type Boolean))
  (`/Engine/EditorBlueprintResources/StandardMacros.FlipFlop`
    (:`A`
      (`self.SetActorHiddenInGame` (`ActorComponent.GetOwner` (`self.PointLight`)) true)
      (`self.SetActorHiddenInGame` (`ActorComponent.GetOwner` (`self.SpotLight`)) true)
      (`self.SetActorHiddenInGame` (`ActorComponent.GetOwner` (`self.SpotLight1`)) true))
    (:`B`
      (`self.SetActorHiddenInGame` (`ActorComponent.GetOwner` (`self.SpotLight1`)) false)
      (`self.SetActorHiddenInGame` (`ActorComponent.GetOwner` (`self.SpotLight`)) false)
      (`self.SetActorHiddenInGame` (`ActorComponent.GetOwner` (`self.PointLight`)) false)))
  (return true))

(fn `UserConstructionScript`)